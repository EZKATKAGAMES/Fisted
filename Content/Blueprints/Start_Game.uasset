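; Start-game actor whose StartCombat event kicks off enemy spawning and breaks apart its destructible DMCube.
; StartCombat starts the EnemySpawner, then applies damage to the cube with a strong impulse, using the actor's location as both hit point and direction.
; After a short delay, a timeline shrinks the cube toward zero scale, lerping from its current scale on each update.
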(event `StartCombat`
  (bind _returnvalue (`self.K2_GetActorLocation`))
  (`/Game/Blueprints/Enemy_Spawner.StartEnemySpawn` (`self.EnemySpawner`))
  (`DestructibleComponent.ApplyDamage` (`self.DM_Cube`) 2.0 _returnvalue _returnvalue 10000.0)
  (`KismetSystemLibrary.Delay` 1.0)
  (bind (_direction _newtrack_0) (`Timeline|Timeline_0` :!via `PlayFromStart`)
    (:`Update`
      (`SceneComponent.SetWorldScale3D` (`self.DM_Cube`) (`KismetMathLibrary.VLerp` (`SceneComponent.K2_GetComponentScale` (`self.DM_Cube`)) (0.0 0.0 0.0) _newtrack_0)))))

(fn `UserConstructionScript`)