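; Melee enemy that chases the player, punches at close range, and reloads the main map when its punch hits the fighter.
; Tick runs a gated AI MoveTo that drives the Anim Blueprint's state and closes on arrival until ChasePlayerAgain reopens it.
; Events toggle the punch collider's overlap detection.
; EnemyDefeated applies damage with a short cooldown, then ragdolls the enemy with directional, upward knockback at zero health.
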(event `EnablePunchCollider`
  (bind _punchcollider (`self.PunchCollider`))
  (`PrimitiveComponent.SetCollisionEnabled` _punchcollider "QueryOnly")
  (`PrimitiveComponent.SetCollisionResponseToAllChannels` _punchcollider "ECR_Overlap"))

(event `self.ReceiveBeginPlay`
  ;[1 1 1] GetAnimationReference
  (bind _asab_enemy (cast `/Game/Blueprints/AnimationBlueprints/AB_Enemy` (`SkeletalMeshComponent.GetAnimInstance` (`self.Mesh`))))
  (set `self.AnimationBlueprintReference` _asab_enemy))

(event `DisablePunchCollider`
  (`PrimitiveComponent.SetCollisionEnabled` (`self.PunchCollider`) "NoCollision"))

(event `self.ReceiveTick`
  (params (DeltaSeconds :type "Float (single-precision)"))
  ;[1 1 1] EventTick
  ;;[1 1 1] MoveToThePlayer
  (`/Engine/EditorBlueprintResources/StandardMacros.Gate` false :!label _label
    (:`Exit`
      (set `/Game/Blueprints/AnimationBlueprints/AB_Enemy.EnemyState` "NewEnumerator1" (`self.AnimationBlueprintReference`))
      (`|AIMoveTo` self (0.0 0.0 0.0) (`GameplayStatics.GetPlayerCharacter` 0) 120.0
        (:`OnSuccess`
          (`|ExecutionSequence`
            (:`then_0`
              ;;[1 1 1] OnlyPunchOncePerSecond
              (`/Engine/EditorBlueprintResources/StandardMacros.DoOnce` false :!label _label_2
                (:`Completed`
                  ;;[1 1 1] PunchPlayerAnimation
                  (set `/Game/Blueprints/AnimationBlueprints/AB_Enemy.EnemyState` "NewEnumerator2" (`self.AnimationBlueprintReference`))
                  (goto _label_2 :!via `Reset`))))
            (:`then_1`
              (goto _label :!via `Close`))))))))

(event `ChasePlayerAgain`
  ;[1 1 1] EventTick
  (goto _label :!via `Open`))

(event `self.PunchCollider.OnComponentBeginOverlap`
  (params (OverlappedComponent :type "PrimitiveComponent Object Reference") (OtherActor :type "Actor Object Reference") (OtherComp :type "PrimitiveComponent Object Reference") (OtherBodyIndex :type Integer) (bFromSweep :type Boolean) (SweepResult :type "HitResult Structure (by ref)"))
  (cast `/Game/Blueprints/BP_FighterCharacter` OtherActor)
  (`GameplayStatics.OpenLevel` "Map_MainGame"))

(event `EnemyDefeated`
  (params (Damage :type Integer) (KnockBackDirection :type "Vector Structure"))
  (bind (_returnvalue_x _returnvalue_y) (`KismetMathLibrary.BreakVector` (* KnockBackDirection (`self.KnockbackAmount`))))
  ;[1 1 1] EnemyDefeated
  (`/Engine/EditorBlueprintResources/StandardMacros.DoOnce` false :!label _label_3
    (:`Completed`
      (set `self.Health` (- (`self.Health`) Damage))
      (`|ExecutionSequence`
        (:`then_0`
          (if (<= (`self.Health`) 0)
            (`/Engine/EditorBlueprintResources/StandardMacros.DoOnce` false
              (:`Completed`
                (`PrimitiveComponent.SetSimulatePhysics` (`self.Mesh`) true)
                (`PrimitiveComponent.SetCollisionEnabled` (`self.CapsuleComponent`) "NoCollision")
                (`PrimitiveComponent.AddImpulse` (`self.Mesh`) (`KismetMathLibrary.MakeVector` _returnvalue_x _returnvalue_y 50000.0) "None" false)))))
        (:`then_1`
          (`KismetSystemLibrary.Delay` 0.4)
          (goto _label_3 :!via `Reset`))))))

(fn `UserConstructionScript`)